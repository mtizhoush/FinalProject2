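; Runner tile, child of a master tile, that randomly populates itself with obstacles, scenery and coins on BeginPlay.
; Three spawn functions each cover their own series of Arrow components, placing trees, bushes and cars in two, and coins or actors with no class shown in the third.
; Nested random rolls form a chain: only a roll of 1 continues to the next arrow, and 0 spawns nothing, so later slots fill less often.
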(event EventBeginPlay
  (CallFunction|SpawnObstacles2)
  (CallFunction|SpawnObstacles)
  (CallFunction|SpawnObstacles3))

(event Collision|EventActorBeginOverlap
  (params (OtherActor :type Actor%20Object%20Reference))
  (|CallParentFunction OtherActor) ; This node is disabled and will not be called.\nDrag off pins to build functionality.
)

(event EventTick
  (params (DeltaSeconds :type Float%20%28single-precision%29))
  (|CallParentFunction DeltaSeconds) ; This node is disabled and will not be called.\nDrag off pins to build functionality.
)

(fn ConstructionScript
  (|CallParentFunction))

(fn SpawnObstacles
  (bind _arrow1 (Variables|Default|GetArrow1))
  (bind _arrow2 (Variables|Default|GetArrow2))
  (bind _arrow3 (Variables|Default|GetArrow3))
  (bind _arrow (Variables|Default|GetArrow))
  (bind _returnvalue (Transformation|GetWorldTransform _arrow1))
  (bind _returnvalue_2 (Transformation|GetWorldTransform _arrow2))
  (bind _returnvalue_3 (Transformation|GetWorldTransform _arrow3))
  (bind _returnvalue_4 (Transformation|GetWorldTransform _arrow))
  (switch int (Math|Random|RandomIntegerinRange 0 3)
    (:1
      (Game|SpawnActorfromClass "/Game/RunnerFiles/BluePrints/BP_Tree.BP_Tree_C" _returnvalue_4 "Undefined" 0 0)
      (switch int (Math|Random|RandomIntegerinRange 0 3)
        (:1
          (Game|SpawnActorfromClass "/Game/RunnerFiles/BluePrints/BP_Tree.BP_Tree_C" _returnvalue "Undefined" 0 0)
          (switch int (Math|Random|RandomIntegerinRange 0 3)
            (:1
              (Game|SpawnActorfromClass "/Game/RunnerFiles/BluePrints/BP_Tree.BP_Tree_C" _returnvalue_2 "Undefined" 0 0)
              (switch int (Math|Random|RandomIntegerinRange 0 2)
                (:1
                  (Game|SpawnActorfromClass "/Game/RunnerFiles/BluePrints/BP_Tree.BP_Tree_C" _returnvalue_3 "Undefined" 0 0))
                (:2
                  (Game|SpawnActorfromClass "/Game/RunnerFiles/BluePrints/BP_Bush.BP_Bush_C" _returnvalue_3 "Undefined" 0 0))))
            (:2
              (Game|SpawnActorfromClass "/Game/RunnerFiles/BluePrints/BP_Bush.BP_Bush_C" _returnvalue_2 "Undefined" 0 0))
            (:3
              (Game|SpawnActorfromClass "/Game/RunnerFiles/BluePrints/Coin.Coin_C" _returnvalue_2 "Undefined" 0 0))))
        (:2
          (Game|SpawnActorfromClass "/Game/RunnerFiles/BluePrints/BP_Bush.BP_Bush_C" _returnvalue "Undefined" 0 0))
        (:3
          (Game|SpawnActorfromClass "/Game/RunnerFiles/BluePrints/Coin.Coin_C" _returnvalue "Undefined" 0 0))))
    (:2
      (Game|SpawnActorfromClass "/Game/RunnerFiles/BluePrints/BP_Bush.BP_Bush_C" _returnvalue_4 "Undefined" 0 0))
    (:3
      (Game|SpawnActorfromClass "/Game/RunnerFiles/BluePrints/Coin.Coin_C" _returnvalue_4 "Undefined" 0 0))))

(fn SpawnObstacles2
  (bind _arrow4 (Variables|Default|GetArrow4))
  (bind _arrow5 (Variables|Default|GetArrow5))
  (bind _arrow6 (Variables|Default|GetArrow6))
  (bind _arrow7 (Variables|Default|GetArrow7))
  (bind _returnvalue (Transformation|GetWorldTransform _arrow5))
  (bind _returnvalue_2 (Transformation|GetWorldTransform _arrow6))
  (bind _returnvalue_3 (Transformation|GetWorldTransform _arrow7))
  (bind _returnvalue_4 (Transformation|GetWorldTransform _arrow4))
  (switch int (Math|Random|RandomIntegerinRange 0 3)
    (:1
      (Game|SpawnActorfromClass "/Game/RunnerFiles/BluePrints/BP_Tree.BP_Tree_C" _returnvalue_4 "Undefined" 0 0)
      (switch int (Math|Random|RandomIntegerinRange 0 3)
        (:1
          (Game|SpawnActorfromClass "/Game/RunnerFiles/BluePrints/BP_Tree.BP_Tree_C" _returnvalue "Undefined" 0 0)
          (switch int (Math|Random|RandomIntegerinRange 0 3)
            (:1
              (Game|SpawnActorfromClass "/Game/RunnerFiles/BluePrints/BP_Tree.BP_Tree_C" _returnvalue_2 "Undefined" 0 0)
              (switch int (Math|Random|RandomIntegerinRange 0 3)
                (:1
                  (Game|SpawnActorfromClass "/Game/RunnerFiles/BluePrints/BP_Tree.BP_Tree_C" _returnvalue_3 "Undefined" 0 0))
                (:2
                  (Game|SpawnActorfromClass "/Game/RunnerFiles/BluePrints/BP_Bush.BP_Bush_C" _returnvalue_3 "Undefined" 0 0))
                (:3
                  (Game|SpawnActorfromClass "/Game/RunnerFiles/BluePrints/BP_Car.BP_Car_C" _returnvalue_3 "Undefined" 0 0))))
            (:2
              (Game|SpawnActorfromClass "/Game/RunnerFiles/BluePrints/BP_Bush.BP_Bush_C" _returnvalue_2 "Undefined" 0 0))
            (:3
              (Game|SpawnActorfromClass "/Game/RunnerFiles/BluePrints/BP_Car.BP_Car_C" _returnvalue_2 "Undefined" 0 0))))
        (:2
          (Game|SpawnActorfromClass "/Game/RunnerFiles/BluePrints/BP_Bush.BP_Bush_C" _returnvalue "Undefined" 0 0))
        (:3
          (Game|SpawnActorfromClass "/Game/RunnerFiles/BluePrints/BP_Car.BP_Car_C" _returnvalue "Undefined" 0 0))))
    (:2
      (Game|SpawnActorfromClass "/Game/RunnerFiles/BluePrints/BP_Bush.BP_Bush_C" _returnvalue_4 "Undefined" 0 0))
    (:3
      (Game|SpawnActorfromClass "/Game/RunnerFiles/BluePrints/BP_Car.BP_Car_C" _returnvalue_4 "Undefined" 0 0))))

(fn SpawnObstacles3
  (bind _arrow8 (Variables|Default|GetArrow8))
  (bind _arrow9 (Variables|Default|GetArrow9))
  (bind _arrow13 (Variables|Default|GetArrow13))
  (bind _arrow10 (Variables|Default|GetArrow10))
  (bind _arrow11 (Variables|Default|GetArrow11))
  (bind _arrow12 (Variables|Default|GetArrow12))
  (bind _returnvalue (Transformation|GetWorldTransform _arrow8))
  (bind _returnvalue_2 (Transformation|GetWorldTransform _arrow13))
  (bind _returnvalue_3 (Transformation|GetWorldTransform _arrow9))
  (bind _returnvalue_4 (Transformation|GetWorldTransform _arrow10))
  (bind _returnvalue_5 (Transformation|GetWorldTransform _arrow11))
  (bind _returnvalue_6 (Transformation|GetWorldTransform _arrow12))
  (switch int (Math|Random|RandomIntegerinRange 0 3)
    (:1
      (Game|SpawnActorfromClass "/Game/RunnerFiles/BluePrints/BP_Tree.BP_Tree_C" _returnvalue "Undefined" 0 0)
      (switch int (Math|Random|RandomIntegerinRange 0 3)
        (:1
          (Game|SpawnActorfromClass "/Game/RunnerFiles/BluePrints/BP_Tree.BP_Tree_C" _returnvalue_3 "Undefined" 0 0)
          (switch int (Math|Random|RandomIntegerinRange 0 3)
            (:1
              (Game|SpawnActorfromClass "/Game/RunnerFiles/BluePrints/BP_Tree.BP_Tree_C" _returnvalue_4 "Undefined" 0 0)
              (switch int (Math|Random|RandomIntegerinRange 0 2)
                (:1
                  (Game|SpawnActorfromClass "/Game/RunnerFiles/BluePrints/BP_Tree.BP_Tree_C" _returnvalue_5 "Undefined" 0 0)
                  (switch int (Math|Random|RandomIntegerinRange 0 2)
                    (:1
                      (Game|SpawnActorfromClass "/Game/RunnerFiles/BluePrints/BP_Tree.BP_Tree_C" _returnvalue_6 "Undefined" 0 0)
                      (switch int (Math|Random|RandomIntegerinRange 0 2)
                        (:1
                          (Game|SpawnActorfromClass "/Game/RunnerFiles/BluePrints/BP_Tree.BP_Tree_C" _returnvalue_2 "Undefined" 0 0))
                        (:2
                          (Game|SpawnActorfromClass "/Game/RunnerFiles/BluePrints/BP_Bush.BP_Bush_C" _returnvalue_2 "Undefined" 0 0))))
                    (:2
                      (Game|SpawnActorfromClass "/Game/RunnerFiles/BluePrints/BP_Bush.BP_Bush_C" _returnvalue_6 "Undefined" 0 0))))
                (:2
                  (Game|SpawnActorfromClass "/Game/RunnerFiles/BluePrints/BP_Bush.BP_Bush_C" _returnvalue_5 "Undefined" 0 0))))
            (:2
              (Game|SpawnActorfromClass "/Game/RunnerFiles/BluePrints/BP_Bush.BP_Bush_C" _returnvalue_4 "Undefined" 0 0))
            (:3
              (Game|SpawnActorfromClass "/Game/RunnerFiles/BluePrints/BP_Car2.BP_Car2_C" _returnvalue_4 "Undefined" 0 0))))
        (:2
          (Game|SpawnActorfromClass "/Game/RunnerFiles/BluePrints/BP_Bush.BP_Bush_C" _returnvalue_3 "Undefined" 0 0))
        (:3
          (Game|SpawnActorfromClass "/Game/RunnerFiles/BluePrints/BP_Car2.BP_Car2_C" _returnvalue_3 "Undefined" 0 0))))
    (:2
      (Game|SpawnActorfromClass "/Game/RunnerFiles/BluePrints/BP_Bush.BP_Bush_C" _returnvalue "Undefined" 0 0))
    (:3
      (Game|SpawnActorfromClass "/Game/RunnerFiles/BluePrints/BP_Car2.BP_Car2_C" _returnvalue "Undefined" 0 0))))